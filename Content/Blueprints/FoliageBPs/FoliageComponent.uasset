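; Component that spawns procedural foliage for actors of a target class and culls foliage by distance from its owner.
; spawnFoliage creates a Foliage actor at the player pawn's location for each target, passing data table rows and a box extent from proceduralHemispheres size and radius.
; UpdateExisting then destroys foliage beyond SpawnDistance, hides the rest beyond HideDistance, and forces garbage collection.
; The overlap check gates nothing, and FoliageData is never cleared between row reads.
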(event Custom|spawnFoliage
  (bind _outactors (Actor|GetAllActorsOfClass (Variables|Default|GetactorToGet)))
  (for _array_element _outactors
    (bind _foliagearray (CallFunction|GetAllRows))
    (if (< (Utilities|Array|Length (Collision|GetOverlappingActors _array_element "/Game/Blueprints/FoliageBPs/Foliage.Foliage_C" :!class /Script/Engine.Actor)) 1)
      _
      (else
        _))
    (bind _returnvalue (Game|SpawnActorfromClass "/Game/Blueprints/FoliageBPs/Foliage.Foliage_C" (Math|Transform|MakeTransform (Transformation|GetActorLocation (Game|Player|GetPlayerPawn 0)) "0, 0, 0" "1,1,1") "Undefined" _array_element _foliagearray (* (* (Variables|/Game/Blueprints/planetBPs/proceduralHemispheres.proceduralHemispheres_C|GetSize (.AsProcedural%20Hemispheres (Utilities|Casting|CastToproceduralHemispheres _array_element))) (Variables|/Game/Blueprints/planetBPs/proceduralHemispheres.proceduralHemispheres_C|GetSize (.AsProcedural%20Hemispheres (Utilities|Casting|CastToproceduralHemispheres _array_element)))) (Variables|/Game/Blueprints/planetBPs/proceduralHemispheres.proceduralHemispheres_C|GetRadius (.AsProcedural%20Hemispheres (Utilities|Casting|CastToproceduralHemispheres _array_element))))))
    ;[1 1 1] handles multiple foliages on object
    (Default|Spawn _returnvalue))
  (CallFunction|UpdateExisting))

(event Custom|UpdateExisting
  ;[1 1 1] checks to see if existing foliages are greater than distance and Hides/Destroys ones above hide distance
  (bind _outactors (Actor|GetAllActorsOfClass "/Game/Blueprints/FoliageBPs/Foliage.Foliage_C"))
  (for _array_element _outactors
    (if (> (Transformation|GetDistanceTo _array_element (Components|GetOwner)) (Variables|Default|GetspawnDistance))
      (Actor|DestroyActor _array_element)
      (else
        (Rendering|SetActorHiddenInGame _array_element (> (Transformation|GetDistanceTo _array_element (Components|GetOwner)) (Variables|Default|GethideDistance))))))
  (Utilities|Platform|CollectGarbage))

(fn GetAllRows
  (bind _outrownames (DataTable|GetDataTableRowNames "/Game/Blueprints/FoliageBPs/FoliageTable.FoliageTable"))
  (for _array_element _outrownames
    (bind _returnvalue (Utilities|GetDataTableRow "/Game/Blueprints/FoliageBPs/FoliageTable.FoliageTable" _array_element)
      (:then
        (Utilities|Array|Add (LocalVariables|GetfoliageData) _returnvalue))))
  (return (LocalVariables|GetfoliageData)))