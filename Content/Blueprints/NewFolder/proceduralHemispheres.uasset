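; Procedural planet Blueprint that builds a noise-displaced sphere, or a plain tiled cube when MakeSphere is off, from its construction script.
; It scales the CubeSides mesh templates, tiling each into a grid of collidable sections on its own Runtime Mesh Component.
; Sphere mode projects vertices onto a radius, displaces them with simplex noise, sets radial normals and rotates eight copies around the planet.
; Only Z-axis faces in sphere mode receive the material.
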(event Custom|generate
  (CallFunction|UpdateQuadSize)
  (if (Variables|Default|GetmakeSphere)
    (for _index (range 0 7)
      (switch int _index
        (:0
          ;[1 1 1] top of planet
          (CallFunction|MakeHemisphere "0,0.000000, 0"))
        (:1
          (CallFunction|MakeHemisphere "0.000000,-90.000000,0.000000"))
        (:2
          (CallFunction|MakeHemisphere "0.000000,90.000000,0.000000"))
        (:3
          (CallFunction|MakeHemisphere "0,180.000000,0.000000"))
        (:4
          ;[1 1 1] bottom half
          (CallFunction|MakeHemisphere "0, 0,90.000000"))
        (:5
          (CallFunction|MakeHemisphere "0,-90.000000,90.000000"))
        (:6
          (CallFunction|MakeHemisphere "0,90.000000,90.000000"))
        (:7
          (CallFunction|MakeHemisphere "0,180.000000,90.000000"))))
    (else
      (CallFunction|MakeHemisphere "0, 0, 0"))))

(event EventBeginPlay)

(fn ConstructionScript
  (CallFunction|Generate))

(fn MakeMeshZ
  (params (MeshData :type Mesh%20Info%20Structure) (RuntimeMesh :type Runtime%20Mesh%20Component%20Object%20Reference))
  (bind (_vertices _triangles) (Utilities|Struct|BreakmeshInfo MeshData))
  (for _index (range 0 (- (* (Variables|Planet|GetSize) (Variables|Planet|GetSize)) 1))
    (bind _returnverts1 (MakeVerts|MakeVertsXY _index _vertices))
    (bind _returnverts1_2 (CallFunction|OffsetVerts _returnverts1))
    (if (Variables|Default|GetmakeSphere)
      (bind _spherified1 (CallFunction|Spherify _returnverts1_2))
      (bind _vertnoise (CallFunction|ApplyNoise _spherified1))
      (bind _normals (CallFunction|NormalizeVerts _vertnoise))
      (Class|RuntimeMeshComponent|CreateMeshSectionBlueprint RuntimeMesh _index _vertnoise _triangles _normals 0 0 0 0 true "Average")
      (Rendering|Material|SetMaterial RuntimeMesh _index (Variables|Planet|GetmaterialInstance))
      (else
        (Class|RuntimeMeshComponent|CreateMeshSectionBlueprint RuntimeMesh _index _returnverts1_2 _triangles 0 0 0 0 0 true "Average")))))

(fn MakeMeshY
  (params (MeshData :type Mesh%20Info%20Structure) (RuntimeMesh :type Runtime%20Mesh%20Component%20Object%20Reference))
  (bind (_vertices _triangles) (Utilities|Struct|BreakmeshInfo MeshData))
  (for _index (range 0 (- (* (Variables|Planet|GetSize) (Variables|Planet|GetSize)) 1))
    (bind _returnverts1 (MakeVerts|MakeVertsYZ _index _vertices))
    (bind _returnverts1_2 (CallFunction|OffsetVerts _returnverts1))
    (if (Variables|Default|GetmakeSphere)
      (bind _spherified1 (CallFunction|Spherify _returnverts1_2))
      (bind _vertnoise (CallFunction|ApplyNoise _spherified1))
      (bind _normals (CallFunction|NormalizeVerts _vertnoise))
      (Class|RuntimeMeshComponent|CreateMeshSectionBlueprint RuntimeMesh _index _vertnoise _triangles _normals 0 0 0 0 true "Average")
      (else
        (Class|RuntimeMeshComponent|CreateMeshSectionBlueprint RuntimeMesh _index _returnverts1_2 _triangles 0 0 0 0 0 true "Average")))))

(fn MakeMeshX
  (params (MeshData :type Mesh%20Info%20Structure) (RuntimeMesh :type Runtime%20Mesh%20Component%20Object%20Reference))
  (bind (_vertices _triangles) (Utilities|Struct|BreakmeshInfo MeshData))
  (for _index (range 0 (- (* (Variables|Planet|GetSize) (Variables|Planet|GetSize)) 1))
    (bind _returnverts1 (MakeVerts|MakeVertsXZ _index _vertices))
    (bind _returnverts1_2 (CallFunction|OffsetVerts _returnverts1))
    (if (Variables|Default|GetmakeSphere)
      (bind _spherified1 (CallFunction|Spherify _returnverts1_2))
      (bind _vertnoise (CallFunction|ApplyNoise _spherified1))
      (bind _normals (CallFunction|NormalizeVerts _vertnoise))
      (Class|RuntimeMeshComponent|CreateMeshSectionBlueprint RuntimeMesh _index _vertnoise _triangles _normals 0 0 0 0 true "Average")
      (else
        (Class|RuntimeMeshComponent|CreateMeshSectionBlueprint RuntimeMesh _index _returnverts1_2 _triangles 0 0 0 0 0 true "Average")))))

(fn MakeVertsXY
  (params (A :type Integer) (Array :type Array%20of%20Vectors))
  (bind _size (Variables|Planet|GetSize))
  (bind _quadsize (Variables|Planet|GetquadSize))
  (for _array_element Array
    (Utilities|Array|Add (LocalVariables|GetreturnVerts) (+ _array_element (Math|Vector|MakeVector (Math|Conversions|ToFloat(Integer) (* (/ A _size) _quadsize)) (Math|Conversions|ToFloat(Integer) (* (Math|Integer|%(Integer) A _size) _quadsize)) (* (- _size 1) (.Z (Math|Vector|BreakVector _array_element)))))))
  (return (LocalVariables|GetreturnVerts)))

(fn OffsetVerts
  (params (Array :type Array%20of%20Vectors) (xOffset :type Integer) (yOffset :type Integer) (zOffset :type Integer))
  (for _array_element Array
    (Utilities|Array|Add (LocalVariables|GetreturnVerts) (* _array_element (Math|Vector|MakeVector (Math|Conversions|ToFloat(Integer) (Math|Integer|Clamp(Integer) xOffset 1 100000)) (Math|Conversions|ToFloat(Integer) (Math|Integer|Clamp(Integer) yOffset 1 100000)) (Math|Conversions|ToFloat(Integer) (Math|Integer|Clamp(Integer) zOffset 1 100000))))))
  (return (LocalVariables|GetreturnVerts)))

(fn MakeVertsXZ
  (params (A :type Integer) (Array :type Array%20of%20Vectors))
  (bind _size (Variables|Planet|GetSize))
  (bind _quadsize (Variables|Planet|GetquadSize))
  (for _array_element Array
    (Utilities|Array|Add (LocalVariables|GetreturnVerts) (+ _array_element (Math|Vector|MakeVector (Math|Conversions|ToFloat(Integer) (* (/ A _size) _quadsize)) (* (- _size 1) (.Y (Math|Vector|BreakVector _array_element))) (Math|Conversions|ToFloat(Integer) (* (Math|Integer|%(Integer) A _size) _quadsize))))))
  (return (LocalVariables|GetreturnVerts)))

(fn MakeVertsYZ
  (params (A :type Integer) (Array :type Array%20of%20Vectors))
  (bind _size (Variables|Planet|GetSize))
  (bind _quadsize (Variables|Planet|GetquadSize))
  (for _array_element Array
    (Utilities|Array|Add (LocalVariables|GetreturnVerts) (+ _array_element (Math|Vector|MakeVector (* (- _size 1) (.X (Math|Vector|BreakVector _array_element))) (Math|Conversions|ToFloat(Integer) (* (/ A _size) _quadsize)) (Math|Conversions|ToFloat(Integer) (* (Math|Integer|%(Integer) A _size) _quadsize))))))
  (return (LocalVariables|GetreturnVerts)))

(fn Spherify
  (params (Vertices :type Array%20of%20Vectors))
  (for _array_element Vertices
    (Utilities|Array|Add (LocalVariables|GetSpherified) (* (* (Math|Vector|Normalize _array_element) (Variables|Planet|GetquadSize)) (Variables|Planet|GetRadius))))
  (return (LocalVariables|GetSpherified)))

(fn NormalizeVerts
  (params (Verts :type Array%20of%20Vectors))
  (for _array_element Verts
    (Utilities|Array|Add (LocalVariables|GetlocNormals) (Math|Vector|Normalize _array_element)))
  (return (LocalVariables|GetlocNormals)))

(fn MakeHemisphere
  (params (Rotation :type Rotator))
  (for (_array_element _array_index) (Variables|Default|GetcubeSides)
    (switch int _array_index
      (:Default
        (return))
      (:0
        ;[1 1 1] inside bit
        (bind _returnvalue (AddComponent|AddRuntimeMeshComponent false))
        (MakeMeshes|MakeMeshZ _array_element _returnvalue)
        (Transformation|SetWorldRotation _returnvalue Rotation false false))
      (:1
        (bind _returnvalue_2 (AddComponent|AddRuntimeMeshComponent false))
        (MakeMeshes|MakeMeshZ _array_element _returnvalue_2)
        (Transformation|SetWorldRotation _returnvalue_2 Rotation false false))
      (:2
        (bind _returnvalue_3 (AddComponent|AddRuntimeMeshComponent false))
        (MakeMeshes|MakeMeshY _array_element _returnvalue_3)
        (Transformation|SetWorldRotation _returnvalue_3 Rotation false false))
      (:3
        ;[1 1 1] inside bit
        (bind _returnvalue_4 (AddComponent|AddRuntimeMeshComponent false))
        (MakeMeshes|MakeMeshY _array_element _returnvalue_4)
        (Transformation|SetWorldRotation _returnvalue_4 Rotation false false))
      (:4
        (bind _returnvalue_5 (AddComponent|AddRuntimeMeshComponent false))
        (MakeMeshes|MakeMeshX _array_element _returnvalue_5)
        (Transformation|SetWorldRotation _returnvalue_5 Rotation false false))
      (:5
        ;[1 1 1] inside bit
        (bind _returnvalue_6 (AddComponent|AddRuntimeMeshComponent false))
        (MakeMeshes|MakeMeshX _array_element _returnvalue_6)
        (Transformation|SetWorldRotation _returnvalue_6 Rotation false false))))
  (return))

(fn UpdateQuadSize
  (bind _newverts (LocalVariables|GetnewVerts))
  (for _array_element (Variables|Default|GetcubeSides)
    (for _array_element_2 (.Vertices (Utilities|Struct|BreakmeshInfo _array_element))
      (Utilities|Array|Add _newverts (* _array_element_2 (Variables|Planet|GetquadSize))))
    (bind _structout (Utilities|Struct|SetmembersinmeshInfo _array_element _newverts))
    (Utilities|Array|Add (LocalVariables|GetnewMeshInfo) _structout)
    (Utilities|Array|Clear (LocalVariables|GetnewVerts)))
  (Variables|Default|SetcubeSides (LocalVariables|GetnewMeshInfo))
  (return))

(fn ApplyNoise
  (params (Array :type Array%20of%20Vectors))
  (for _array_element Array
    (bind _returnvalue (Class|SimplexNoiseBPLibrary|SimplexNoiseScaled3D (.Y (Math|Vector|BreakVector _array_element)) (.X (Math|Vector|BreakVector _array_element)) (.Z (Math|Vector|BreakVector _array_element)) (Variables|Planet|Noise|GetNoiseScale)))
    (Utilities|Array|Add (LocalVariables|GetupdatedVerts) (Math|Vector|Lerp(Vector) _array_element (* _array_element _returnvalue) (Variables|Planet|Noise|GetNoiseIntensity))))
  (return (LocalVariables|GetupdatedVerts)))