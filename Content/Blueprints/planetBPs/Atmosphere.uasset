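; Planet atmosphere actor that procedurally builds a spherical shell from runtime mesh components, generated in the construction script when RunInEditor is set.
; Generate scales eight octant datasets by QuadSize, then MakeHemisphere tiles selected faces of each into Size-by-Size sections.
; With MakeSphere on, vertices are normalized and scaled into a cube-sphere with radial normals and the atmosphere material.
; The construction script also writes the SunLight's forward vector to the MPC_SunDirection parameter collection.
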(event Custom|generate
  (CallFunction|UpdateQuadSize (Variables|Default|Gethemisphere2))
  (CallFunction|UpdateQuadSize (Variables|Default|Gethemisphere3))
  (CallFunction|UpdateQuadSize (Variables|Default|Gethemisphere1))
  (CallFunction|UpdateQuadSize (Variables|Default|Gethemisphere4))
  (CallFunction|UpdateQuadSize (Variables|Default|Gethemisphere5))
  (CallFunction|UpdateQuadSize (Variables|Default|Gethemisphere6))
  (CallFunction|UpdateQuadSize (Variables|Default|Gethemisphere7))
  (CallFunction|UpdateQuadSize (Variables|Default|Gethemisphere8))
  (if (Variables|Default|GetmakeSphere)
    _
    (else
      _))
  (for _index (range 0 7)
    (switch int _index
      (:0
        ;[1 1 1] top of planet
        (CallFunction|MakeHemisphere "0,0.000000, 0" (Variables|Default|Gethemisphere1)))
      (:1
        (CallFunction|MakeHemisphere "0.000000,0.000000,0.000000" (Variables|Default|Gethemisphere2)))
      (:2
        (CallFunction|MakeHemisphere "0.000000,0.000000,0.000000" (Variables|Default|Gethemisphere3)))
      (:3
        (CallFunction|MakeHemisphere "0,0.000000,0.000000" (Variables|Default|Gethemisphere4)))
      (:4
        ;[1 1 1] bottom half
        (CallFunction|MakeHemisphere "0.000000,0.000000,0.000000" (Variables|Default|Gethemisphere5)))
      (:5
        (CallFunction|MakeHemisphere "0.000000,0.000000,0.000000" (Variables|Default|Gethemisphere6)))
      (:6
        (CallFunction|MakeHemisphere "0.000000,0.000000,0.000000" (Variables|Default|Gethemisphere7)))
      (:7
        (CallFunction|MakeHemisphere "0.000000,0.000000,0.000000" (Variables|Default|Gethemisphere8))))))

(event EventBeginPlay)

(fn ConstructionScript
  (if (Variables|Default|GetRun%20In%20Editor)
    (CallFunction|Generate)
    (if (Variables|Default|GetRefresh%20Sun)
      (Variables|Default|SetRefresh%20Sun false))
    (Rendering|Material|SetVectorParameterValue "/Game/Blueprints/planetBPs/PlanetMat/Atmosphere/MPC_SunDirection.MPC_SunDirection" "LightDirection" (Math|Conversions|ToLinearColor(Vector) (Math|Rotator|GetRotationXVector (Transformation|GetActorRotation (Variables|Default|GetSun%20Light)))) :!class /Script/Engine.KismetMaterialLibrary)))

(fn MakeMeshZ
  (params (MeshData :type Mesh%20Info%20Structure) (RuntimeMesh :type Runtime%20Mesh%20Component%20Object%20Reference))
  (bind (_vertices _triangles) (Utilities|Struct|BreakmeshInfo MeshData))
  (for _index (range 0 (* (Variables|Planet|GetSize) (Variables|Planet|GetSize)))
    (bind _returnverts1 (MakeVerts|MakeVertsXY _index _vertices))
    (if (Variables|Default|GetmakeSphere)
      (bind _spherified1 (CallFunction|Spherify _returnverts1))
      (bind _normals (CallFunction|NormalizeVerts _spherified1))
      (Class|RuntimeMeshComponent|CreateMeshSectionBlueprint RuntimeMesh _index _spherified1 _triangles _normals 0 0 0 0 false "Average")
      (Rendering|Material|SetMaterial RuntimeMesh _index (Variables|Planet|GetmaterialInstance))
      (else
        (Class|RuntimeMeshComponent|CreateMeshSectionBlueprint RuntimeMesh _index _returnverts1 _triangles 0 0 0 0 0 false "Average")))))

(fn MakeMeshY
  (params (MeshData :type Mesh%20Info%20Structure) (RuntimeMesh :type Runtime%20Mesh%20Component%20Object%20Reference))
  (bind (_vertices _triangles) (Utilities|Struct|BreakmeshInfo MeshData))
  (for _index (range 0 (* (Variables|Planet|GetSize) (Variables|Planet|GetSize)))
    (bind _returnverts1 (MakeVerts|MakeVertsYZ _index _vertices))
    (if (Variables|Default|GetmakeSphere)
      (bind _spherified1 (CallFunction|Spherify _returnverts1))
      (bind _normals (CallFunction|NormalizeVerts _spherified1))
      (Class|RuntimeMeshComponent|CreateMeshSectionBlueprint RuntimeMesh _index _spherified1 _triangles _normals 0 0 0 0 false "Average")
      (Rendering|Material|SetMaterial RuntimeMesh _index (Variables|Planet|GetmaterialInstance))
      (else
        (Class|RuntimeMeshComponent|CreateMeshSectionBlueprint RuntimeMesh _index _returnverts1 _triangles 0 0 0 0 0 false "Average")))))

(fn MakeMeshX
  (params (MeshData :type Mesh%20Info%20Structure) (RuntimeMesh :type Runtime%20Mesh%20Component%20Object%20Reference))
  (bind (_vertices _triangles) (Utilities|Struct|BreakmeshInfo MeshData))
  (for _index (range 0 (* (Variables|Planet|GetSize) (Variables|Planet|GetSize)))
    (bind _returnverts1 (MakeVerts|MakeVertsXZ _index _vertices))
    (if (Variables|Default|GetmakeSphere)
      (bind _spherified1 (CallFunction|Spherify _returnverts1))
      (bind _normals (CallFunction|NormalizeVerts _spherified1))
      (Class|RuntimeMeshComponent|CreateMeshSectionBlueprint RuntimeMesh _index _spherified1 _triangles _normals 0 0 0 0 false "Average")
      (Rendering|Material|SetMaterial RuntimeMesh _index (Variables|Planet|GetmaterialInstance))
      (else
        (Class|RuntimeMeshComponent|CreateMeshSectionBlueprint RuntimeMesh _index _returnverts1 _triangles 0 0 0 0 0 false "Average")))))

(fn MakeVertsXY
  (params (A :type Integer) (Array :type Array%20of%20Vectors))
  (bind _size (Variables|Planet|GetSize))
  (bind _quadsize (Variables|Planet|GetquadSize))
  (for _array_element Array
    (Utilities|Array|Add (LocalVariables|GetreturnVerts) (+ _array_element (Math|Vector|MakeVector (Math|Conversions|ToFloat(Integer) (* (/ A _size) _quadsize)) (Math|Conversions|ToFloat(Integer) (* (Math|Integer|%(Integer) A _size) _quadsize)) (* (- _size 1) (.Z (Math|Vector|BreakVector _array_element)))))))
  (return (LocalVariables|GetreturnVerts)))

(fn OffsetVerts
  (params (Array :type Array%20of%20Vectors) (xOffset :type Integer) (yOffset :type Integer) (zOffset :type Integer))
  (for _array_element Array
    (Utilities|Array|Add (LocalVariables|GetreturnVerts) (* _array_element (Math|Vector|MakeVector (Math|Conversions|ToFloat(Integer) (Math|Integer|Clamp(Integer) xOffset 1 100000)) (Math|Conversions|ToFloat(Integer) (Math|Integer|Clamp(Integer) yOffset 1 100000)) (Math|Conversions|ToFloat(Integer) (Math|Integer|Clamp(Integer) zOffset 1 100000))))))
  (return (LocalVariables|GetreturnVerts)))

(fn MakeVertsXZ
  (params (A :type Integer) (Array :type Array%20of%20Vectors))
  (bind _size (Variables|Planet|GetSize))
  (bind _quadsize (Variables|Planet|GetquadSize))
  (for _array_element Array
    (Utilities|Array|Add (LocalVariables|GetreturnVerts) (+ _array_element (Math|Vector|MakeVector (Math|Conversions|ToFloat(Integer) (* (/ A _size) _quadsize)) (* (- _size 1) (.Y (Math|Vector|BreakVector _array_element))) (Math|Conversions|ToFloat(Integer) (* (Math|Integer|%(Integer) A _size) _quadsize))))))
  (return (LocalVariables|GetreturnVerts)))

(fn MakeVertsYZ
  (params (A :type Integer) (Array :type Array%20of%20Vectors))
  (bind _size (Variables|Planet|GetSize))
  (bind _quadsize (Variables|Planet|GetquadSize))
  (for _array_element Array
    (Utilities|Array|Add (LocalVariables|GetreturnVerts) (+ _array_element (Math|Vector|MakeVector (* (- _size 1) (.X (Math|Vector|BreakVector _array_element))) (Math|Conversions|ToFloat(Integer) (* (/ A _size) _quadsize)) (Math|Conversions|ToFloat(Integer) (* (Math|Integer|%(Integer) A _size) _quadsize))))))
  (return (LocalVariables|GetreturnVerts)))

(fn Spherify
  (params (Vertices :type Array%20of%20Vectors))
  (for _array_element Vertices
    (Utilities|Array|Add (LocalVariables|GetSpherified) (* (* (Math|Vector|Normalize _array_element) (Variables|Planet|GetquadSize)) (Variables|Planet|GetRadius))))
  (return (LocalVariables|GetSpherified)))

(fn NormalizeVerts
  (params (Verts :type Array%20of%20Vectors))
  (for _array_element Verts
    (Utilities|Array|Add (LocalVariables|GetlocNormals) (Math|Vector|Normalize _array_element)))
  (return (LocalVariables|GetlocNormals)))

(fn MakeHemisphere
  (params (Rotation :type Rotator) (CubeData :type Array%20of%20Mesh%20Info%20Structures))
  (for (_array_element _array_index) CubeData
    (switch int _array_index
      (:Default
        (return))
      (:1
        (bind _returnvalue (AddComponent|AddRuntimeMeshComponent false))
        (MakeMeshes|MakeMeshZ _array_element _returnvalue)
        (Transformation|SetWorldRotation _returnvalue Rotation false false))
      (:2
        (bind _returnvalue_2 (AddComponent|AddRuntimeMeshComponent false))
        (MakeMeshes|MakeMeshY _array_element _returnvalue_2)
        (Transformation|SetWorldRotation _returnvalue_2 Rotation false false))
      (:4
        (bind _returnvalue_3 (AddComponent|AddRuntimeMeshComponent false))
        (MakeMeshes|MakeMeshX _array_element _returnvalue_3)
        (Transformation|SetWorldRotation _returnvalue_3 Rotation false false))))
  (return))

(fn UpdateQuadSize
  (params (MeshInfo :type Array%20of%20Mesh%20Info%20Structures))
  (bind _newverts (LocalVariables|GetnewVerts))
  (for _array_element MeshInfo
    (for _array_element_2 (.Vertices (Utilities|Struct|BreakmeshInfo _array_element))
      (Utilities|Array|Add _newverts (* _array_element_2 (Variables|Planet|GetquadSize))))
    (bind _structout (Utilities|Struct|SetmembersinmeshInfo _array_element _newverts))
    (Utilities|Array|Add (LocalVariables|GetnewMeshInfo) _structout)
    (Utilities|Array|Clear (LocalVariables|GetnewVerts)))
  (Utilities|Array|Clear MeshInfo)
  (Utilities|Array|AppendArray MeshInfo (LocalVariables|GetnewMeshInfo))
  (return))