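; Planet actor that composes a procedurally generated planet and its surrounding atmosphere from two child actors, a proceduralHemispheres and an Atmosphere.
; When Generate is set, the construction script casts both children, copies shared seed, size, noise, radius and material settings into them, and triggers their generation.
; The atmosphere radius is offset by DistanceFromPlanet, and its scaled radius is written to the MPC_SunDirection parameter collection as PlanetScale.
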(event `initPlanetData`
  ;[1 1 1] Setup References
  (set `self.PlanetRef` (cast `/Game/Blueprints/planetBPs/proceduralHemispheres` (`ChildActorComponent.ChildActor` (`self.planet`)) :!pure true))
  (set `self.AtmosphereRef` (cast `/Game/Blueprints/planetBPs/Atmosphere` (`ChildActorComponent.ChildActor` (`self.atmosphere`)) :!pure true))
  (`self.InitializePlanetData`)
  (`self.InitializeAtmosphereData`))

(fn `InitializeAtmosphereData`
  (bind _atmosphereref (`self.AtmosphereRef`))
  (set `/Game/Blueprints/planetBPs/Atmosphere.planetSeed` (`self.Seed`) _atmosphereref)
  (bind _output_get (set `/Game/Blueprints/planetBPs/Atmosphere.Size` (`self.Size`) _atmosphereref))
  (set `/Game/Blueprints/planetBPs/Atmosphere.quadSize` (`self.QuadSize`) _atmosphereref)
  (bind _output_get_2 (set `/Game/Blueprints/planetBPs/Atmosphere.Radius` (+ (`self.Radius`) (`self.DistanceFromPlanet`)) _atmosphereref))
  (set `/Game/Blueprints/planetBPs/Atmosphere.materialInstance` (`self.AtmosphereMat`) _atmosphereref)
  (set `/Game/Blueprints/planetBPs/Atmosphere.Sun Light` null _atmosphereref)
  (`/Game/Blueprints/planetBPs/Atmosphere.generate` _atmosphereref)
  (`KismetMaterialLibrary.SetScalarParameterValue` "/Game/Blueprints/planetBPs/PlanetMat/Atmosphere/MPC_SunDirection.MPC_SunDirection" "PlanetScale" (* _output_get _output_get_2))
  (return))

(fn `InitializePlanetData`
  (bind _planetref (`self.PlanetRef`))
  (set `/Game/Blueprints/planetBPs/proceduralHemispheres.planetSeed` (`self.Seed`) _planetref)
  (set `/Game/Blueprints/planetBPs/proceduralHemispheres.Size` (`self.Size`) _planetref)
  (set `/Game/Blueprints/planetBPs/proceduralHemispheres.quadSize` (`self.QuadSize`) _planetref)
  (set `/Game/Blueprints/planetBPs/proceduralHemispheres.NoiseScale` (`self.NoiseScale`) _planetref)
  (set `/Game/Blueprints/planetBPs/proceduralHemispheres.NoiseIntensity` (`self.NoiseIntensity`) _planetref)
  (set `/Game/Blueprints/planetBPs/proceduralHemispheres.Noise Smoothing` (`self.NoiseSmoothness`) _planetref)
  (set `/Game/Blueprints/planetBPs/proceduralHemispheres.PlanetMaterial` (`self.PlanetMat`) _planetref)
  (set `/Game/Blueprints/planetBPs/proceduralHemispheres.Radius` (`self.Radius`) _planetref)
  (`/Game/Blueprints/planetBPs/proceduralHemispheres.generate` _planetref)
  (return))

(fn `UserConstructionScript`
  (if (`self.Generate`)
    (`self.initPlanetData`)))