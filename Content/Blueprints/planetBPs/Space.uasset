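; Space Blueprint that rotates a directional light as a moving sun and shares its direction with materials.
; A looping one-second timer started on BeginPlay steps the light's local rotation, then writes its forward vector to the LightDirection parameter of the MPC_SunDirection material parameter collection.
; The construction script makes the same parameter write, syncing the direction to the light's placed rotation without rotating it.
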(event `self.ReceiveBeginPlay`
  (`KismetSystemLibrary.K2_SetTimerDelegate` (delegate `updateSunRotation`) 1.0 true))

(event `updateSunRotation`
  (bind _directionallight (`self.DirectionalLight`))
  (`SceneComponent.K2_AddLocalRotation` _directionallight (struct :`Pitch` 1.0 :`Yaw` 5.0 :`Roll` 5.0) false false)
  (`KismetMaterialLibrary.SetVectorParameterValue` "/Game/Blueprints/planetBPs/PlanetMat/Atmosphere/MPC_SunDirection.MPC_SunDirection" "LightDirection" (`KismetMathLibrary.Conv_VectorToLinearColor` (`KismetMathLibrary.Conv_RotatorToVector` (`SceneComponent.K2_GetComponentRotation` _directionallight)))))

(fn `UserConstructionScript`
  (`KismetMaterialLibrary.SetVectorParameterValue` "/Game/Blueprints/planetBPs/PlanetMat/Atmosphere/MPC_SunDirection.MPC_SunDirection" "LightDirection" (`KismetMathLibrary.Conv_VectorToLinearColor` (`KismetMathLibrary.Conv_RotatorToVector` (`SceneComponent.K2_GetComponentRotation` (`self.DirectionalLight`))))))