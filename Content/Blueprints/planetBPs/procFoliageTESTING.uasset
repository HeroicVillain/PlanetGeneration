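; Test Blueprint for procedural foliage placement on a grid, currently unfinished and spawning nothing.
; The construction script runs spawnGrid, which loads FoliageTable rows into FoliageData and loops over a count derived from the owner's X and Y bounds extents.
; Each iteration increments a local seed for a repeatable random roll, but the result leads nowhere; grid position and mesh selection nodes are unconnected.
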(event Custom|spawnGrid
  (bind _returnvalue (Components|GetOwner))
  (bind _boxextent (Collision|GetActorBounds _returnvalue true))
  (bind (_x _y) (Math|Vector|BreakVector _boxextent))
  (Variables|Private|SetlocalSeed (Variables|Default|GetSeed))
  (bind _output_get (Variables|Default|SetmaxX _x))
  (bind _output_get_2 (Variables|Default|SetmaxY _y))
  (bind _foliagedata1 (CallFunction|GetFoliage))
  (for _index (range 0 (Math|Float|Truncate (- (* _output_get _output_get_2) 1.0)))
    (Math|Integer|IncrementInt (Variables|Private|GetlocalSeed)
      (:%20%20
        (if (== (Math|Random|RandomIntegerinRangefromStream -1 (Utilities|Array|Length _foliagedata1) (Math|Random|MakeRandomStream (Variables|Private|GetlocalSeed))) -1)
          _)))))

(event EventBeginPlay)

(event Collision|EventActorBeginOverlap
  (params (OtherActor :type Actor%20Object%20Reference)))

(event EventTick
  (params (DeltaSeconds :type Float%20%28single-precision%29)))

(fn ConstructionScript
  (CallFunction|SpawnGrid))

(fn GetFoliage
  (bind _outrownames (DataTable|GetDataTableRowNames "/Game/Blueprints/FoliageBPs/FoliageTable.FoliageTable"))
  (for _array_element _outrownames
    (bind _returnvalue (Utilities|GetDataTableRow "/Game/Blueprints/FoliageBPs/FoliageTable.FoliageTable" _array_element)
      (:then
        (Utilities|Array|Add (LocalVariables|GetfoliageData) _returnvalue))))
  (return (LocalVariables|GetfoliageData)))